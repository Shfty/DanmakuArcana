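; Editor-style visualizer actor that previews shmup bullet pattern trajectories as persistent red debug lines from its construction script.
; When Load is set, it copies spawner and bullet data from a pattern table row, otherwise it uses its current values.
; For each bullet set and stream, it steps IntegrateBullet at high or low tick rate, applying spawner rotation each step.
; Simulation stops at bullet lifespan or MaxDuration, whichever is shorter.
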(event EventBeginPlay)

(event Collision|EventActorBeginOverlap
  (params (OtherActor :type Actor%20Object%20Reference)))

(event EventTick
  (params (DeltaSeconds :type Float%20%28single-precision%29)))

(fn ConstructionScript
  (bind _returnvalue (Transformation|GetActorLocation))
  (bind _highprecisiontickrate (Variables|BulletTrajectoryVisualizer|Simulation|GetHighPrecisionTickRate))
  (bind _usehighprecision (Variables|BulletTrajectoryVisualizer|GetUseHighPrecision))
  (bind _lowprecisiontickrate (Variables|BulletTrajectoryVisualizer|Simulation|GetLowPrecisionTickRate))
  (bind _returnvalue_2 (Math|Integer|SelectInt _highprecisiontickrate _lowprecisiontickrate _usehighprecision))
  (bind _returnvalue_3 (Math|Conversions|ToFloat(Integer) _returnvalue_2))
  (bind _returnvalue_4 (/ 1.0 _returnvalue_3))
  (if (Variables|BulletTrajectoryVisualizer|LoadFromDataTable|GetLoad)
    (bind _returnvalue_5 (Utilities|GetDataTableRow "/Game/Shmup/Data/PatternTable.PatternTable" (Utilities|Struct|BreakDataTableRowHandle (Variables|BulletTrajectoryVisualizer|LoadfromDataTable|GetSourceRow)))
      (:then
        (Variables|BulletTrajectoryVisualizer|PatternData|SetSpawnerData (.SpawnerData (Utilities|Struct|BreakPatternData _returnvalue_5)))
        (Variables|BulletTrajectoryVisualizer|PatternData|SetBulletData (.BulletData (Utilities|Struct|BreakPatternData _returnvalue_5))))))
  (Rendering|Debug|FlushPersistentDebugLines)
  (for _array_element (.BulletSets (Utilities|Struct|BreakShmupSpawnerData (Variables|BulletTrajectoryVisualizer|PatternData|GetSpawnerData)))
    (for _index (range 0 (- (.BulletStreams (Utilities|Struct|BreakShmupSpawnerData (Variables|BulletTrajectoryVisualizer|PatternData|GetSpawnerData))) 1))
      (LocalVariables|SetTimeAccumulator 0.0)
      (LocalVariables|SetLocalTransform (Math|Transform|MakeTransform "0, 0, 0" (Math|Rotator|CombineRotators (CallFunction|CalculateBulletStreamRotation (.BulletStreams (Utilities|Struct|BreakShmupSpawnerData (Variables|BulletTrajectoryVisualizer|PatternData|GetSpawnerData))) _index (Variables|BulletTrajectoryVisualizer|PatternData|GetSpawnerData)) _array_element)))
      (LocalVariables|SetLocalBulletData (Variables|BulletTrajectoryVisualizer|PatternData|GetBulletData))
      (while (< (LocalVariables|GetTimeAccumulator) (Math|Float|Min(Float) (Utilities|Struct|BreakShmupBulletData (Variables|BulletTrajectoryVisualizer|PatternData|GetBulletData)) (Variables|BulletTrajectoryVisualizer|Simulation|GetMaxDuration)))
        (bind (_integratedtransform _integrateddata) (CallFunction|IntegrateBullet (LocalVariables|GetLocalTransform) (LocalVariables|GetLocalBulletData) _returnvalue_4))
        (Rendering|Debug|DrawDebugLine (+ (.Location (Math|Transform|BreakTransform (LocalVariables|GetLocalTransform))) _returnvalue) (+ (.Location (Math|Transform|BreakTransform (Math|Transform|MakeTransform (Math|Vector|RotateVectorAroundAxis (.Location (Math|Transform|BreakTransform _integratedtransform)) (* (Utilities|Struct|BreakShmupSpawnerData (Variables|BulletTrajectoryVisualizer|PatternData|GetSpawnerData)) _returnvalue_4) "0, 0,-1.000000") (Math|Rotator|CombineRotators (.Rotation (Math|Transform|BreakTransform _integratedtransform)) (Math|Vector|RotatorfromAxisandAngle "0, 0,-1.000000" (* (Utilities|Struct|BreakShmupSpawnerData (Variables|BulletTrajectoryVisualizer|PatternData|GetSpawnerData)) _returnvalue_4))) (.Scale (Math|Transform|BreakTransform _integratedtransform))))) _returnvalue) "(R=1.000000,G=0.000000,B=0.000000,A=1.000000)" 1e+04 0.0)
        (LocalVariables|SetLocalTransform (Math|Transform|MakeTransform (Math|Vector|RotateVectorAroundAxis (.Location (Math|Transform|BreakTransform _integratedtransform)) (* (Utilities|Struct|BreakShmupSpawnerData (Variables|BulletTrajectoryVisualizer|PatternData|GetSpawnerData)) _returnvalue_4) "0, 0,-1.000000") (Math|Rotator|CombineRotators (.Rotation (Math|Transform|BreakTransform _integratedtransform)) (Math|Vector|RotatorfromAxisandAngle "0, 0,-1.000000" (* (Utilities|Struct|BreakShmupSpawnerData (Variables|BulletTrajectoryVisualizer|PatternData|GetSpawnerData)) _returnvalue_4))) (.Scale (Math|Transform|BreakTransform _integratedtransform))))
        (LocalVariables|SetLocalBulletData _integrateddata)
        (LocalVariables|SetTimeAccumulator (+ (LocalVariables|GetTimeAccumulator) _returnvalue_4))
        (Math|Integer|IncrementInt (LocalVariables|GetNumSteps))))))
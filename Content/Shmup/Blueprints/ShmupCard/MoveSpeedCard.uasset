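; MoveSpeedCard is a shmup card that changes the owning pawn's movement speed while the card is active.
; Activation and deactivation call the parent handlers, then SetPawnSpeedModifier.
; That function sets the owning pawn's MoveSpeed to BaseMoveSpeed times SpeedMultiplier, or back to BaseMoveSpeed when inactive, so it overwrites rather than stacks with other speed changes.
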(event EventActivatedInternal
  (params (ActivationLocation :type Vector :default "0, 0, 0"))
  (|CallParentFunction ActivationLocation)
  (CallFunction|SetPawnSpeedModifier true))

(event EventDeactivatedInternal
  (params (DeactivationLocation :type Vector :default "0, 0, 0"))
  (|CallParentFunction DeactivationLocation)
  (CallFunction|SetPawnSpeedModifier false))

(fn SetPawnSpeedModifier
  (params (Active :type Boolean))
  (bind (_owningpawn _success) (CallFunction|GetOwningPawn))
  (bind _basemovespeed (Variables|/Game/Shmup/Blueprints/GameplayFramework/Pawn/BattlePawn.BattlePawn_C|GetBaseMoveSpeed _owningpawn))
  (if _success
    (Variables|/Game/Shmup/Blueprints/GameplayFramework/Pawn/BattlePawn.BattlePawn_C|SetMoveSpeed _owningpawn (Math|Float|SelectFloat (* _basemovespeed (Variables|Default|GetSpeedMultiplier)) _basemovespeed Active))))
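; Base card component for a shmup battle pawn that spends player Power on activation and restores it on release, handling networking for child cards.
; Pawn input passes overridable Can checks, adjusts Power immediately on the local player, and sends the owner's location to the server.
; An optional ping-based delay precedes setting the location locally.
; Location RepNotifies run the empty internal effect hooks and adjust Power on non-local copies.
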(event Custom|ActivateReleased
  ;[1 1 1] Deactivation handlers
  (if (CallFunction|CanDeactivate)
    (CallFunction|Deactivated)))

(event Custom|TakePower
  (bind (_owningpawn _success) (CallFunction|GetOwningPawn))
  (bind (_shmupplayerstate _success_2) (Default|GetPlayerState _owningpawn))
  (if _success
    (if _success_2
      (Default|ModifyPower _shmupplayerstate (* (Variables|Default|GetPowerCost) -1)))))

(event Custom|ClientDeactivateOnServer
  (params (DeactivationLocation :type Vector))
  ;[1 1 1] Deactivation handlers
  (Variables|Replication|SetDeactivationLocation DeactivationLocation))

(event Custom|Deactivated
  ;[1 1 1] Deactivation handlers
  (Variables|Default|SetCachedDeactivationLocation (Transformation|GetActorLocation (Components|GetOwner)))
  (Utilities|FlowControl|Sequence
    (:then_0
      (Utilities|SwitchLocallyControlled
        (:Local
          (CallFunction|RestorePower))))
    (:then_1
      (Utilities|SwitchHasAuthority
        (:Remote
          (CallFunction|ClientDeactivateonServer (Variables|Default|GetCachedDeactivationLocation)))))
    (:then_2
      (if (Variables|Default|GetUseActivationDelay)
        (Utilities|FlowControl|Delay (CallFunction|CalculatePingDelayTime (.ShmupPlayerState (Default|GetPlayerState (.OwningPawn (CallFunction|GetOwningPawn)))))))
      (Variables|Replication|SetDeactivationLocation (Variables|Default|GetCachedDeactivationLocation)))))

(event Custom|ActivatePressed
  ;[1 1 1] Activation handlers
  (if (CallFunction|CanActivate)
    (CallFunction|Activated)))

(event Custom|Activated
  ;[1 1 1] Activation handlers
  (Variables|Default|SetCachedActivationLocation (Transformation|GetActorLocation (Components|GetOwner)))
  (Utilities|FlowControl|Sequence
    (:then_0
      (Utilities|SwitchLocallyControlled
        (:Local
          (CallFunction|TakePower))))
    (:then_1
      (Utilities|SwitchHasAuthority
        (:Remote
          (CallFunction|ClientActivateonServer (Variables|Default|GetCachedActivationLocation)))))
    (:then_2
      (if (Variables|Default|GetUseActivationDelay)
        (Utilities|FlowControl|Delay (CallFunction|CalculatePingDelayTime (.ShmupPlayerState (Default|GetPlayerState (.OwningPawn (CallFunction|GetOwningPawn)))))))
      (Variables|Replication|SetActivationLocation (Variables|Default|GetCachedActivationLocation)))))

(event Custom|RestorePower
  (bind (_owningpawn _success) (CallFunction|GetOwningPawn))
  (bind (_shmupplayerstate _success_2) (Default|GetPlayerState _owningpawn))
  (if _success
    (if _success_2
      (Default|ModifyPower _shmupplayerstate (Variables|Default|GetPowerCost)))))

(event Custom|ClientActivateOnServer
  (params (ActivationLocation :type Vector))
  ;[1 1 1] Activation handlers
  (Variables|Replication|SetActivationLocation ActivationLocation))

(event Custom|FixedTick
  (params (DeltaTime :type Float%20%28single-precision%29) (TickCount :type Integer)))

(fn GetOwningPawn
  (bind _asbattle_pawn (Utilities|Casting|CastToBattlePawn (Components|GetOwner))
    (:then
      (return _asbattle_pawn true))
    (:CastFailed
      (return 0 false))))

(fn ActivatedInternal
  (params (ActivationLocation :type Vector)))

(fn DeactivatedInternal
  (params (DeactivationLocation :type Vector)))

(fn CanActivate
  (bind (_owningpawn _success) (CallFunction|GetOwningPawn))
  (bind (_shmupplayerstate _success_2) (Default|GetPlayerState _owningpawn))
  (if _success
    (if _success_2
      (return (>= (Variables|/Game/Shmup/Blueprints/GameplayFramework/PlayerState/BattlePlayerState.BattlePlayerState_C|GetPower _shmupplayerstate) (Variables|Default|GetPowerCost)))
      (else
        _)))
  (return false))

(fn CanDeactivate
  (return true))

(fn OnRepActivationLocation
  (CallFunction|ActivatedInternal (Variables|Replication|GetActivationLocation))
  (Utilities|SwitchLocallyControlled
    (:Remote
      (CallFunction|TakePower))))

(fn OnRepDeactivationLocation
  (CallFunction|DeactivatedInternal (Variables|Replication|GetDeactivationLocation))
  (Utilities|SwitchLocallyControlled
    (:Remote
      (CallFunction|RestorePower))))
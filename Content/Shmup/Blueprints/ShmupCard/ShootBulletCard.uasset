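; ShootBulletCard is a shmup card that fires bullets from its owning pawn while the card is active.
; Activation and deactivation set and clear a ShootPressed flag after calling the parent logic.
; On each fixed tick, if the pawn is in the required mode and the tick count is a multiple of FireRate, the global bullet manager spawns a bullet at the pawn's transform using the card's data, mesh and material.
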(event EventActivatedInternal
  (params (ActivationLocation :type Vector :default "0, 0, 0"))
  (|CallParentFunction ActivationLocation)
  (Variables|Default|SetShootPressed true))

(event EventDeactivatedInternal
  (params (DeactivationLocation :type Vector :default "0, 0, 0"))
  (|CallParentFunction DeactivationLocation)
  (Variables|Default|SetShootPressed false))

(event EventFixedTick
  (params (DeltaTime :type Float%20%28single-precision%29) (TickCount :type Integer))
  (bind (_owningpawn _success) (CallFunction|GetOwningPawn))
  (if _success
    (if (Math|Boolean|ANDBoolean (Utilities|Enum|Equal(Enum) (Variables|/Game/Shmup/Blueprints/GameplayFramework/Pawn/BattlePawn.BattlePawn_C|GetMode _owningpawn) "NewEnumerator0") (== (Math|Integer|%(Integer) TickCount (Variables|Default|GetFireRate)) 0) (Variables|Default|GetShootPressed))
      (Default|SpawnBullet (.GlobalBulletManager (CallFunction|GetGlobalBulletManager)) (Transformation|GetActorTransform _owningpawn) (Variables|Default|GetBulletData) (Variables|Default|GetBulletMesh) (Variables|Default|GetBulletMaterial)))))
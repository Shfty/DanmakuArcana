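; Shmup card that casts a bullet pattern by spawning a bullet spawner at the activation location, optionally aimed at the opposing player's pawn.
; It takes its display name from the pattern row and activates only in a specific match phase and pawn mode, with no spawner alive.
; Once the spawner is gone, fixed ticks count down an optional cooldown before deactivating.
; Manual deactivation is disallowed, while forced deactivation destroys any live spawner.
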(event EventFixedTick
  (params (DeltaTime :type Float%20%28single-precision%29) (TickCount :type Integer))
  (bind _cooldownframes (Variables|Default|GetCooldownFrames))
  (|CallParentFunction DeltaTime TickCount)
  (if (Variables|Default|GetIsActivated)
    (Utilities|IsValid (Variables|Default|GetBulletSpawner)
      (:Is%20Not%20Valid
        (if (== (Variables|Default|GetCooldownTimer) -1)
          (if (> _cooldownframes 0)
            (Variables|Default|SetCooldownTimer _cooldownframes)
            (else
              (CallFunction|Deactivated :!label _label)
              (Variables|Default|SetCooldownTimer -1)))
          (elif (> (Variables|Default|GetCooldownTimer) 0)
            (bind _result (Math|Integer|DecrementInt (Variables|Default|GetCooldownTimer))
              (:%20%20
                (if (== _result 0)
                  (goto _label))))))))))

(event EventActivatedInternal
  (params (ActivationLocation :type Vector :default "0, 0, 0"))
  (bind (_owningpawn _success) (CallFunction|GetOwningPawn))
  (bind (_shmupplayerstate _success_2) (Default|GetPlayerState _owningpawn))
  (|CallParentFunction ActivationLocation)
  (if _success
    (if _success_2
      (bind _returnvalue (Game|SpawnActorfromClass "/Game/Shmup/Blueprints/Bullets/Spawning/ShmupBulletSpawner.ShmupBulletSpawner_C" (Math|Transform|MakeTransform ActivationLocation (Math|Rotator|SelectRotator (Math|Rotator|FindLookatRotation (Transformation|GetActorLocation _owningpawn) (Transformation|GetActorLocation (.Pawn (CallFunction|FindBattlePawnforSide (Utilities|Select :Index (Variables|/Game/Shmup/Blueprints/GameplayFramework/PlayerState/BattlePlayerState.BattlePlayerState_C|GetSide _shmupplayerstate) :NewEnumerator5 "NewEnumerator5" :NewEnumerator0 "NewEnumerator7" :NewEnumerator7 "NewEnumerator0"))))) "0, 0, 0" (Variables|Default|GetIsAimed))) "AlwaysSpawn" _owningpawn (Variables|Default|GetPattern) _owningpawn))
      (Variables|Default|SetBulletSpawner _returnvalue))))

(event EventBeginPlay
  (Variables|Default|SetDisplayName (Utilities|Text|ToText(Name) (.RowName (Utilities|Struct|BreakDataTableRowHandle (Variables|Default|GetPattern))))))

(event EventDeactivatedInternal
  (params (DeactivationLocation :type Vector :default "0, 0, 0"))
  (bind _bulletspawner (Variables|Default|GetBulletSpawner))
  (|CallParentFunction DeactivationLocation)
  ;[1 1 1] Destroy bullet spawner if it's valid in case this is a forced deactivation
  (Utilities|IsValid _bulletspawner
    (:Is%20Valid
      (Actor|DestroyActor _bulletspawner))))

(fn CanActivate
  (bind (_shmup_game_state _success) (CallFunction|GetBattleGameState))
  (bind (_owningpawn _success_2) (CallFunction|GetOwningPawn))
  (if (and _success_2 _success)
    (return (Math|Boolean|ANDBoolean (Utilities|Enum|Equal(Enum) (Variables|/Game/Shmup/Blueprints/GameplayFramework/GameState/BattleGameState.BattleGameState_C|GetMatchPhase _shmup_game_state) "NewEnumerator2") (Utilities|Enum|Equal(Enum) (Variables|/Game/Shmup/Blueprints/GameplayFramework/Pawn/BattlePawn.BattlePawn_C|GetMode _owningpawn) "NewEnumerator7") (not (Utilities|IsValid (Variables|Default|GetBulletSpawner))) (|CallParentFunction)))))

(fn CanDeactivate
  (return false))
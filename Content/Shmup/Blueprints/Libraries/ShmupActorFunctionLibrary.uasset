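; Blueprint function library of shared helpers for a two-sided networked shmup battle.
; Bullet helpers step transform, velocity and lifespan from pattern data, and fan stream rotations evenly across a spawner cone.
; Delay helpers subtract half the player's ping frames from client-side event timing, converting to seconds with the fixed tick manager's timestep.
; Other functions fetch battle framework objects, flip side or mode enums, perform map travel and set UI focus.
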(fn IntegrateBullet
  (params (BulletTransform :type Transform) (PatternData :type Pattern%20Data%20Structure) (DeltaTime :type Float%20%28single-precision%29))
  (bind (_bullet_linearvelocity _bullet_linearacceleration _bullet_angularvelocity _bullet_angularacceleration _bullet_lifespan) (Utilities|Struct|BreakPatternData PatternData))
  (bind (_location _rotation _scale) (Math|Transform|BreakTransform BulletTransform))
  (bind _structout (Utilities|Struct|SetmembersinPatternData PatternData (+ _bullet_linearvelocity (* _bullet_linearacceleration DeltaTime)) (+ _bullet_angularvelocity (* _bullet_angularacceleration DeltaTime)) (Math|Float|SelectFloat (Math|Float|Max(Float) (- _bullet_lifespan DeltaTime) 0.0) -1.0 (> _bullet_lifespan 0.0))))
  (return (Math|Transform|MakeTransform (+ _location (* (Math|Vector|GetForwardVector _rotation) (* _bullet_linearvelocity DeltaTime))) (Math|Rotator|CombineRotators (Math|Vector|RotatorfromAxisandAngle "0, 0,1.000000" (* _bullet_angularvelocity DeltaTime)) _rotation) _scale) _structout))

(fn GetFixedTickManager
  (bind _outactors (Actor|GetAllActorsOfClass 0 "/Game/FixedTick/FixedTickManager.FixedTickManager_C"))
  (if (> (Utilities|Array|Length _outactors) 0)
    (return (Utilities|Array|Get(acopy) _outactors) (Variables|/Game/FixedTick/FixedTickManager.FixedTickManager_C|GetFixedTickComponent (Utilities|Array|Get(acopy) _outactors)))
    (else
      (return 0 0))))

(fn GetGlobalBulletManager
  (bind _asbattle_game_state (Utilities|Casting|CastToBattleGameState (Game|GetGameState))
    (:then
      (return (Variables|/Game/Shmup/Blueprints/GameplayFramework/GameState/BattleGameState.BattleGameState_C|GetGlobalBulletManager _asbattle_game_state) true))
    (:CastFailed
      (return 0 true))))

(fn CalculateBulletStreamRotation
  (params (StreamCount :type Integer) (StreamIndex :type Integer) (PatternData :type Pattern%20Data%20Structure%20%28by%20ref%29))
  (bind _spawner_conehalfangle (Utilities|Struct|BreakPatternData PatternData))
  (return (Math|Vector|RotatorfromAxisandAngle "0, 0,1.000000" (- (* StreamIndex (/ (* _spawner_conehalfangle 2.0) (Math|Conversions|ToFloat(Integer) (Math|Integer|Max(Integer) (- StreamCount 1) 1)))) (Math|Float|SelectFloat _spawner_conehalfangle 0.0 (> StreamCount 1))))))

(fn GetBattleGameState
  (bind _asbattle_game_state (Utilities|Casting|CastToBattleGameState (Game|GetGameState))
    (:then
      (return _asbattle_game_state true))
    (:CastFailed
      (return 0 false))))

(fn CalculateEventDelayTime
  (params (Delay :type Float%20%28single-precision%29) (PlayerState :type Battle%20Player%20State%20Object%20Reference))
  (return Delay (- Delay (CallFunction|CalculatePingDelayTime PlayerState))))

(fn CalculatePingDelayTime
  (params (PlayerState :type Battle%20Player%20State%20Object%20Reference))
  (return (* (CallFunction|CalculatePingDelayFrames PlayerState) (Variables|/Game/FixedTick/FixedTickComponent.FixedTickComponent_C|GetTimestep (Variables|/Game/FixedTick/FixedTickManager.FixedTickManager_C|GetFixedTickComponent (.FixedTickManager (CallFunction|GetFixedTickManager)))))))

(fn GetBattlePlayerState
  (bind _returnvalue (Game|GetPlayerController 0))
  (bind _playerstate (Variables|/Script/Engine.Controller|GetPlayerState _returnvalue))
  (bind (_asbattle_player_state _bsuccess) (Utilities|Casting|CastToBattlePlayerState _playerstate))
  (return _asbattle_player_state _bsuccess))

(fn CalculatePingDelayFrames
  (params (PlayerState :type Battle%20Player%20State%20Object%20Reference))
  (Utilities|IsValid PlayerState
    (:Is%20Valid
      (return (/ (Variables|/Game/Shmup/Blueprints/GameplayFramework/PlayerState/BattlePlayerState.BattlePlayerState_C|GetPingFrames PlayerState) 2)))
    (:Is%20Not%20Valid
      (return 0))))

(fn CalculateEventDelayFrames
  (params (DelayFrames :type Integer) (PlayerState :type Battle%20Player%20State%20Object%20Reference))
  (Utilities|IsValid PlayerState
    (:Is%20Valid
      (return DelayFrames (- DelayFrames (CallFunction|CalculatePingDelayFrames PlayerState))))))

(fn GetShmupGameInstance
  (bind _asshmup_game_instance (Utilities|Casting|CastToShmupGameInstance (Game|GetGameInstance))
    (:then
      (return _asshmup_game_instance true))
    (:CastFailed
      (return 0 false))))

(fn ServerTravel
  (params (Map :type String) (Mode :type String) (SeamlessTravel :type Boolean) (Listen :type Boolean))
  (Development|ExecuteConsoleCommand 0 (Utilities|String|Append (Utilities|String|SelectString "ServerTravel" "open" SeamlessTravel) " " Map (Utilities|String|Append (Utilities|String|SelectString "?game=" "" (Utilities|Enum|NotEqual(Enum) Mode "")) Mode) (Utilities|String|SelectString "?listen" "" Listen))))

(fn SetUserFocusConditional
  (params (PlayerController :type Player%20Controller%20Object%20Reference) (WidgetToFocus :type Widget%20Object%20Reference))
  (if (not (Class|Widget|HasFocusedDescendants WidgetToFocus))
    (Class|DanmakuArcanaStatics|SetUserFocus PlayerController WidgetToFocus)))

(fn GetBattleGameMode
  (bind _asbattle_game_mode (Utilities|Casting|CastToBattleGameMode (Game|GetGameMode))
    (:then
      (return _asbattle_game_mode true))
    (:CastFailed
      (return 0 false))))

(fn GetGlobalPlayArea
  (bind _asbattle_game_state (Utilities|Casting|CastToBattleGameState (Game|GetGameState))
    (:then
      (return (Variables|/Game/Shmup/Blueprints/GameplayFramework/GameState/BattleGameState.BattleGameState_C|GetGlobalPlayArea _asbattle_game_state) true))
    (:CastFailed
      (return 0 false))))

(fn GetOpposingSide
  (params (NewParam :type ShmupPawnSide%20Enum :default "NewEnumerator5"))
  (return (Utilities|Select :Index NewParam :NewEnumerator5 "NewEnumerator5" :NewEnumerator0 "NewEnumerator7" :NewEnumerator7 "NewEnumerator0")))

(fn GetOpposingMode
  (params (Index :type ShmupPawnMode%20Enum :default "NewEnumerator5"))
  (return (Utilities|Select :Index Index :NewEnumerator5 "NewEnumerator5" :NewEnumerator0 "NewEnumerator7" :NewEnumerator7 "NewEnumerator0")))
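; Blueprint function library of helpers for the shmup's widgets, covering player lookup by side and UI key checks.
; Battle player state, battle pawn and lobby player state lookups scan all actors of the class and return the first matching Side, with pawns matched through their player state.
; Battle lookups reject one specific Side enum value up front.
; Key predicates map keyboard and gamepad buttons to profile panel up, back and delete, plus main UI back.
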(fn FindBattlePlayerStateforSide
  (params (Side :type ShmupPawnSide%20Enum :default "NewEnumerator5"))
  (if (Utilities|Enum|NotEqual(Enum) Side "NewEnumerator5")
    (bind _outactors (Actor|GetAllActorsOfClass 0 "/Game/Shmup/Blueprints/GameplayFramework/PlayerState/BattlePlayerState.BattlePlayerState_C"))
    (for _array_element _outactors
      (if (Utilities|Enum|Equal(Enum) (Variables|/Game/Shmup/Blueprints/GameplayFramework/PlayerState/BattlePlayerState.BattlePlayerState_C|GetSide _array_element) Side)
        (return _array_element true))))
  (return 0 false))

(fn FindBattlePawnforSide
  (params (Side :type ShmupPawnSide%20Enum :default "NewEnumerator5"))
  (if (Utilities|Enum|NotEqual(Enum) Side "NewEnumerator5")
    (bind _outactors (Actor|GetAllActorsOfClass 0 "/Game/Shmup/Blueprints/GameplayFramework/Pawn/BattlePawn.BattlePawn_C"))
    (for _array_element _outactors
      (if (.Success (Default|GetPlayerState _array_element))
        (if (Utilities|Enum|Equal(Enum) (Variables|/Game/Shmup/Blueprints/GameplayFramework/PlayerState/BattlePlayerState.BattlePlayerState_C|GetSide (.ShmupPlayerState (Default|GetPlayerState _array_element))) Side)
          (return _array_element true)))))
  (return 0 false))

(fn FindLobbyPlayerStateforSide
  (params (Side :type ShmupPawnSide%20Enum :default "NewEnumerator5"))
  (bind _outactors (Actor|GetAllActorsOfClass 0 "/Game/Shmup/Blueprints/GameplayFramework/PlayerState/LobbyPlayerState.LobbyPlayerState_C"))
  (for _array_element _outactors
    (if (Utilities|Enum|Equal(Enum) (Variables|/Game/Shmup/Blueprints/GameplayFramework/PlayerState/LobbyPlayerState.LobbyPlayerState_C|GetSide _array_element) Side)
      (return _array_element)))
  (return 0))

(fn KeyIsProfilePanelUp
  (params (InputPin :type Key%20Structure))
  (return (or (== InputPin "Tab") (== InputPin "Gamepad_Special_Left"))))

(fn KeyIsProfilePanelBack
  (params (InputPin :type Key%20Structure))
  (return (or (== InputPin "Escape") (== InputPin "Gamepad_FaceButton_Right"))))

(fn KeyIsMainUIBack
  (params (Key :type Key%20Structure))
  (return (or (== Key "Escape") (== Key "Gamepad_FaceButton_Right"))))

(fn KeyIsProfilePanelDelete
  (params (InputPin :type Key%20Structure))
  (return (or (== InputPin "Delete") (== InputPin "Gamepad_FaceButton_Top"))))
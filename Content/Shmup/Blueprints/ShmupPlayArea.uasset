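; Shmup play area actor that defines a flat rectangular boundary from an Extent around its location.
; Construction script flushes persistent debug lines and redraws the white outline, and BeginPlay draws it again with a very long duration.
; IsPointWithinPlayArea tests a point's X and Y offsets against Extent, ignoring Z.
; The test uses world axes, while the drawn box follows actor rotation.
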(event EventBeginPlay
  (bind _extent (Variables|Default|GetExtent))
  (bind (_x _y) (Math|Vector2D|BreakVector2D _extent))
  (Rendering|Debug|DrawDebugBox (Transformation|GetActorLocation) (Math|Vector|MakeVector _x _y 0.0) "(R=1.000000,G=1.000000,B=1.000000,A=1.000000)" (Transformation|GetActorRotation) 1e+06 0.0))

(fn ConstructionScript
  (bind _extent (Variables|Default|GetExtent))
  (bind (_x _y) (Math|Vector2D|BreakVector2D _extent))
  (Rendering|Debug|FlushPersistentDebugLines)
  (Rendering|Debug|DrawDebugBox (Transformation|GetActorLocation) (Math|Vector|MakeVector _x _y 0.0) "(R=1.000000,G=1.000000,B=1.000000,A=1.000000)" (Transformation|GetActorRotation) 1e+06 0.0))

(fn IsPointWithinPlayArea
  (params (Point :type Vector))
  (bind _returnvalue (Transformation|GetActorLocation))
  (bind _extent (Variables|Default|GetExtent))
  (bind _returnvalue_2 (- Point _returnvalue))
  (bind (_x _y) (Math|Vector2D|BreakVector2D _extent))
  (bind (_x_2 _y_2) (Math|Vector|BreakVector _returnvalue_2))
  (return (and (<= (Math|Float|Absolute(Float) _x_2) _x) (<= (Math|Float|Absolute(Float) _y_2) _y))))